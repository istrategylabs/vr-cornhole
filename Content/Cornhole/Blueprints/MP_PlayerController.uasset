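; Multiplayer player controller for Cornhole that gives a player a VR thrower pawn after login.
; ClientPostLogin hands off to ServerRespawnMe, a client-to-server split suggested by the event names.
; The respawn destroys any currently controlled pawn, spawns a VR_Pawn_Thrower owned by the controller at a hardcoded transform regardless of collision, then possesses it and enables its input.
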(event `Client Post Login`
  ;[1 1 1] Client-side respawn
  (`self.Server Respawn Me`))

(event `Server Respawn Me`
  (bind _returnvalue (`self.K2_GetPawn`))
  ;[0.794 1 0.3074] Server Respawn
  (`/Engine/EditorBlueprintResources/StandardMacros.IsValid` _returnvalue
    (:`Is Valid`
      (`self.K2_DestroyActor` _returnvalue))
    (:`Is Not Valid`
      _))
  (bind _returnvalue_2 (`|SpawnActorFromClass` "/Game/Cornhole/Blueprints/VR_Pawn_Thrower.VR_Pawn_Thrower_C" (`KismetMathLibrary.MakeTransform` (-1390.0 0.0 20.0)) "AlwaysSpawn" "OverrideRootScale" self))
  (`self.Possess` _returnvalue_2)
  (`self.EnableInput` _returnvalue_2 self))

(fn `UserConstructionScript`)