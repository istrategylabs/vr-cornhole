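; VR pawn for a cornhole game that lets the player pick up and throw sacks with motion-controller hands.
; The right-hand reach trigger highlights a sack via custom depth, and the trigger input grabs or releases it, toggling ownership and physics.
; Tick snaps held sacks to grip points and passes movement through Replicate events, applying the right-hand transform only on non-locally-controlled pawns.
; It also enables the HMD and offers a debug level reset.
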(event `self.R_ReachTrigger.OnComponentBeginOverlap`
  (params (OverlappedComponent :type "PrimitiveComponent Object Reference") (OtherActor :type "Actor Object Reference") (OtherComp :type "PrimitiveComponent Object Reference") (OtherBodyIndex :type Integer) (bFromSweep :type Boolean) (SweepResult :type "HitResult Structure (by ref)"))
  ;[1 1 1] Right-Hand Reach Overlap Begin
  (bind _asbp_sack (cast `/Game/Cornhole/Blueprints/BP_Sack` OtherActor))
  (set `self.R_Sacks In Range` _asbp_sack)
  (`PrimitiveComponent.SetRenderCustomDepth` (`/Game/Cornhole/Blueprints/BP_Sack.SackMesh` _asbp_sack) true))

(event `self.R_ReachTrigger.OnComponentEndOverlap`
  (params (OverlappedComponent :type "PrimitiveComponent Object Reference") (OtherActor :type "Actor Object Reference") (OtherComp :type "PrimitiveComponent Object Reference") (OtherBodyIndex :type Integer))
  ;[1 1 1] Right-Hand Reach Overlap End
  (bind _asbp_sack (cast `/Game/Cornhole/Blueprints/BP_Sack` OtherActor))
  (set `self.R_Sacks In Range` null)
  (`PrimitiveComponent.SetRenderCustomDepth` (`/Game/Cornhole/Blueprints/BP_Sack.SackMesh` _asbp_sack) false))

(event `InputAction|R_Trigger`
  (params (Key :type "Key Structure" :default "AnyKey"))
  ;[1 1 1] Right-Hand Grip Hold
  (:`Pressed`
    (`ActorComponent.SetActive` (`self.R_ReachTrigger`) false false)
    (bind _output_get (set `self.R_Sacks in Grip` (`self.R_Sacks In Range`)))
    (set `self.R_Sacks In Range` null)
    (bind _asbp_sack (cast `/Game/Cornhole/Blueprints/BP_Sack` _output_get))
    (`self.SetOwner` _asbp_sack self)
    (`self.Replicate Sack Physics Toggle` false _asbp_sack)))

(event `InputAction|R_Trigger`
  (params (Key :type "Key Structure" :default "AnyKey"))
  (bind _r_sacks_in_grip (`self.R_Sacks in Grip`))
  ;[1 1 1] Right-Hand Grip Release
  (:`Released`
    (`ActorComponent.SetActive` (`self.R_ReachTrigger`) true false)
    (`/Engine/EditorBlueprintResources/StandardMacros.IsValid` _r_sacks_in_grip
      (:`Is Valid`
        (bind _asbp_sack (cast `/Game/Cornhole/Blueprints/BP_Sack` _r_sacks_in_grip))
        (`self.SetOwner` _asbp_sack null)
        (`self.Replicate Sack Physics Toggle` true _asbp_sack)
        ;;[1 1 1] Just in case clear this out again
        (set `self.R_Sacks in Grip` null)
        (set `self.R_Sacks In Range` null)))))

(event `self.ReceiveTick`
  (params (DeltaSeconds :type "Float (single-precision)"))
  (bind _l_sacks_in_grip (`self.L_Sacks in Grip`))
  (bind _r_sacks_in_grip (`self.R_Sacks in Grip`))
  (`self.Replicate Right Hand` (`SceneComponent.K2_GetComponentToWorld` (`self.R_HandMesh`)))
  ;[1 1 1] Right-Hand
  (`/Engine/EditorBlueprintResources/StandardMacros.IsValid` _r_sacks_in_grip
    (:`Is Valid`
      (bind _asbp_sack (cast `/Game/Cornhole/Blueprints/BP_Sack` _r_sacks_in_grip)
        (:`then`
          (`self.Replicate Sack Movement` (.location (`SceneComponent.K2_GetComponentToWorld` (`self.R_GripPoint`))) (.rotation (`SceneComponent.K2_GetComponentToWorld` (`self.R_GripPoint`))) _asbp_sack))
        (:`CastFailed`
          _)))
    (:`Is Not Valid`
      _))
  ;[1 1 1] Right-Hand
  (`/Engine/EditorBlueprintResources/StandardMacros.IsValid` _l_sacks_in_grip
    (:`Is Valid`
      (bind _asbp_sack_2 (cast `/Game/Cornhole/Blueprints/BP_Sack` _l_sacks_in_grip))
      (`self.Replicate Sack Movement` (.location (`SceneComponent.K2_GetComponentToWorld` (`self.L_GripPoint`))) (.rotation (`SceneComponent.K2_GetComponentToWorld` (`self.L_GripPoint`))) _asbp_sack_2))))

(event `InputAction|Debug_Reset`
  (params (Key :type "Key Structure" :default "AnyKey"))
  ;[1 1 1] Reset Level
  (:`Pressed`
    (bind _returnvalue (`GameplayStatics.GetCurrentLevelName` true))
    (`GameplayStatics.OpenLevel` (`KismetStringLibrary.Conv_StringToName` _returnvalue))))

(event `self.ReceiveBeginPlay`
  ;[1 1 1] Enable HMD
  (`HeadMountedDisplayFunctionLibrary.EnableHMD` true))

(event `Replicate Sack Movement`
  (params (Loc :type "Vector Structure") (Rot :type "Rotator Structure") (Sack :type "/Game/Cornhole/Blueprints/BP_Sack Object Reference"))
  (`SceneComponent.K2_SetWorldLocationAndRotation` (`/Game/Cornhole/Blueprints/BP_Sack.SackMesh` Sack) Loc Rot false false))

(event `Replicate Sack Physics Toggle`
  (params (`Is Simulating Physics` :type Boolean) (Sack :type "/Game/Cornhole/Blueprints/BP_Sack Object Reference"))
  (`PrimitiveComponent.SetSimulatePhysics` (`/Game/Cornhole/Blueprints/BP_Sack.SackMesh` Sack) `Is Simulating Physics`))

(event `Replicate Right Hand`
  (params (Transform :type "Transform Structure"))
  (if (not (`self.IsLocallyControlled`))
    (`SceneComponent.K2_SetWorldTransform` (`self.R_HandMesh`) Transform false false)))

(fn `UserConstructionScript`)