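; VR menu handler for the Cornhole game that lets the right motion controller point at and click a 3D menu.
; It enables the HMD on BeginPlay, then line traces forward from the right hand every tick.
; Hits on components whose names start with "3DMenu" toggle cursor visibility, while a hit menu actor receives the impact location.
; Right trigger presses are forwarded to the child-actor menu while it is targeted.
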(event `InputAction|R_Trigger`
  (params (Key :type "Key Structure" :default "AnyKey"))
  (bind _3dmenu (`self.3DMenu`))
  (:`Pressed`
    (if (`self.Menu Was Hit`)
      (`/Engine/EditorBlueprintResources/StandardMacros.IsValid` _3dmenu
        (:`Is Valid`
          (bind _as3dmenu (cast `/Game/Cornhole/Blueprints/3DMenu` (`ChildActorComponent.ChildActor` _3dmenu)))
          (`/Game/Cornhole/Blueprints/3DMenu.Trigger Pulled On Menu` _as3dmenu))))))

(event `self.ReceiveBeginPlay`
  (`HeadMountedDisplayFunctionLibrary.EnableHMD` true))

(event `self.ReceiveTick`
  (params (DeltaSeconds :type "Float (single-precision)"))
  (`self.HandleLineTraceForMenu`))

(fn `HandleLineTraceForMenu`
  (bind (_outposition _outorientation) (`SteamVRFunctionLibrary.GetHandPositionAndOrientation` 0 "Right"))
  (bind _returnvalue (+ _outposition (`self.K2_GetActorLocation`)))
  (bind _outhit (`KismetSystemLibrary.LineTraceSingleForObjects` :`Start` _returnvalue :`End` (+ _returnvalue (* (`KismetMathLibrary.GetForwardVector` _outorientation) 3000.0)) :`ObjectTypes` (`|MakeArray` "ObjectTypeQuery2" :!type "EObjectTypeQuery Enum") :`TraceColor` (struct :`G` 0.079631 :`B` 1.0 :`A` 1.0)))
  (bind (_bblockinghit _binitialoverlap _time _location _impactpoint _normal _impactnormal _physmat _hitactor _hitcomponent) (`GameplayStatics.BreakHitResult` _outhit))
  (set `self.Impact Location` _impactpoint)
  (bind _as3dmenu (cast `/Game/Cornhole/Blueprints/3DMenu` (`ChildActorComponent.ChildActor` (`self.3DMenu`)))
    (:`then`
      (bind _returnvalue_2 (`KismetStringLibrary.StartsWith` (`KismetSystemLibrary.GetDisplayName` _hitcomponent) "3DMenu"))
      (`/Game/Cornhole/Blueprints/3DMenu.Update Cursor Visibility` _as3dmenu _returnvalue_2))
    (:`CastFailed`
      _))
  (set `self.Menu Was Hit` _returnvalue_2)
  (bind _as3dmenu_2 (cast `/Game/Cornhole/Blueprints/3DMenu` _hitactor)
    (:`then`
      (`/Game/Cornhole/Blueprints/3DMenu.RaytraceWorldLocation` _as3dmenu_2 (`self.Impact Location`)))
    (:`CastFailed`
      _))
  (return))

(fn `UserConstructionScript`)