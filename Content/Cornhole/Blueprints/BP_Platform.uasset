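; BP_Platform is the cornhole board that scores thrown BP_Sack actors and shows the total on a text render.
; Two trigger volumes count overlapping sacks: each one in the over trigger scores one point, each in the under trigger scores triple.
; Any begin or end overlap on either trigger recounts from the current overlaps, so the score follows sacks entering and leaving without a stored running total.
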(event `self.Under_Trigger.OnComponentBeginOverlap`
  (params (OverlappedComponent :type "PrimitiveComponent Object Reference") (OtherActor :type "Actor Object Reference") (OtherComp :type "PrimitiveComponent Object Reference") (OtherBodyIndex :type Integer) (bFromSweep :type Boolean) (SweepResult :type "HitResult Structure (by ref)"))
  (bind _points (`self.CountPoints`))
  (`self.SetScoreText` _points))

(event `self.Under_Trigger.OnComponentEndOverlap`
  (params (OverlappedComponent :type "PrimitiveComponent Object Reference") (OtherActor :type "Actor Object Reference") (OtherComp :type "PrimitiveComponent Object Reference") (OtherBodyIndex :type Integer))
  (bind _points (`self.CountPoints`))
  (`self.SetScoreText` _points))

(event `self.Over_Trigger.OnComponentBeginOverlap`
  (params (OverlappedComponent :type "PrimitiveComponent Object Reference") (OtherActor :type "Actor Object Reference") (OtherComp :type "PrimitiveComponent Object Reference") (OtherBodyIndex :type Integer) (bFromSweep :type Boolean) (SweepResult :type "HitResult Structure (by ref)"))
  (bind _points (`self.CountPoints`))
  (`self.SetScoreText` _points))

(event `self.Over_Trigger.OnComponentEndOverlap`
  (params (OverlappedComponent :type "PrimitiveComponent Object Reference") (OtherActor :type "Actor Object Reference") (OtherComp :type "PrimitiveComponent Object Reference") (OtherBodyIndex :type Integer))
  (bind _points (`self.CountPoints`))
  (`self.SetScoreText` _points))

(fn `CountPoints`
  (returns (Points :type Integer))
  (bind _count (`self.CountTopPoints`))
  (bind _count_2 (`self.CountUnderPoints`))
  (return (+ _count _count_2)))

(fn `CountTopPoints`
  (returns (Count :type Integer))
  (return (`KismetArrayLibrary.Array_Length` (`PrimitiveComponent.GetOverlappingActors` (`self.Over_Trigger`) "/Game/Cornhole/Blueprints/BP_Sack.BP_Sack_C"))))

(fn `CountUnderPoints`
  (returns (Count :type Integer))
  (return (* (`KismetArrayLibrary.Array_Length` (`PrimitiveComponent.GetOverlappingActors` (`self.Under_Trigger`) "/Game/Cornhole/Blueprints/BP_Sack.BP_Sack_C")) 3)))

(fn `SetScoreText`
  (params (Score :type Integer))
  (`TextRenderComponent.K2_SetText` (`self.TextRender`) (`KismetTextLibrary.Conv_IntToText` Score)))

(fn `UserConstructionScript`)