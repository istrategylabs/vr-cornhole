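; Game instance for the Cornhole game that tracks a current game-state enum and handles showing the main menu.
; An IsCurrentState macro branches on whether a given state matches the current one.
; BeginPlayShowMainMenu fires ShowMainMenuEvent from one enum state, and that event opens the MainMenu level only in another state.
; TransitionToState only checks the desired state and never assigns it.
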(event `ShowMainMenuEvent`
  (`self.IsCurrentState` "NewEnumerator5"
    (:`True`
      (`GameplayStatics.OpenLevel` "MainMenu"))))

(fn `BeginPlay Show Main Menu`
  (`self.IsCurrentState` "NewEnumerator0"
    (:`True`
      (`self.ShowMainMenuEvent`))))