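; 3D menu actor for Cornhole that hosts the MainMenu widget in the world and relays pointer and trigger input to it.
; Incoming world-space raytrace locations are converted into the widget component's local space and negated before being passed to the menu.
; Cursor visibility changes and trigger pulls are forwarded to the menu, with a trigger pull acting as a button click.
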(event `RaytraceWorldLocation`
  (params (Location :type "Vector Structure"))
  (bind _widget (`self.Widget`))
  (bind _asmain_menu (cast `/Game/Cornhole/User_Interfaces/MainMenu` (`WidgetComponent.GetUserWidgetObject` _widget)))
  (`/Game/Cornhole/User_Interfaces/MainMenu.RaytraceWidgetLocation` _asmain_menu (* (`KismetMathLibrary.InverseTransformLocation` (`SceneComponent.K2_GetComponentToWorld` _widget) Location) -1.0)))

(event `Update Cursor Visibility`
  (params (Visibility :type Boolean))
  (bind _asmain_menu (cast `/Game/Cornhole/User_Interfaces/MainMenu` (`WidgetComponent.GetUserWidgetObject` (`self.Widget`))))
  (`/Game/Cornhole/User_Interfaces/MainMenu.Update Cursor Visibility` _asmain_menu Visibility))

(event `Trigger Pulled On Menu`
  (bind _asmain_menu (cast `/Game/Cornhole/User_Interfaces/MainMenu` (`WidgetComponent.GetUserWidgetObject` (`self.Widget`))))
  (`/Game/Cornhole/User_Interfaces/MainMenu.Button Clicked` _asmain_menu))

(fn `UserConstructionScript`)